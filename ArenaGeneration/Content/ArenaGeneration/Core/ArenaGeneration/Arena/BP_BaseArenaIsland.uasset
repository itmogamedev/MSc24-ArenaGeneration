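; Base actor for an island in the generated arena, which builds its floor geometry with Geometry Script.
; When generation finishes, it extrudes each polygon and height pair from ExtrudeData into the FloorDynamicMesh component.
; It then recomputes UVs and normals, applies a material set and generates collision from the resulting mesh.
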(event EventBeginPlay)

(event Collision|EventActorBeginOverlap
  (params (OtherActor :type Actor%20Object%20Reference)))

(event EventTick
  (params (DeltaSeconds :type Float%20%28single-precision%29)))

(event EventGenerationFinished
  (bind _floordynamicmesh (Variables|Default|GetFloorDynamicMesh))
  (bind _returnvalue (DynamicMeshComponent|GetDynamicMesh (Variables|Default|GetFloorDynamicMesh)))
  (for _array_element (Variables|Default|GetExtrudeData)
    (Class|GeometryScriptLibraryMeshPrimitiveFunctions|AppendSimpleExtrudePolygon :TargetMesh _returnvalue :PolygonVertices (.vertices _array_element) :Height (.height _array_element) :Debug 0))
  (bind _returnvalue_2 (Class|GeometryScriptLibraryMeshUVFunctions|RecomputeMeshUVs :TargetMesh _returnvalue :Options (Variables|Default|GetOptions) :Debug 0))
  (bind _returnvalue_3 (GeometryScript|Normals|RecomputeNormals :TargetMesh _returnvalue_2 :Debug 0))
  (Class|DynamicMeshComponent|ConfigureMaterialSet _floordynamicmesh (Variables|Default|GetNew%20Material%20Set))
  (Class|GeometryScriptLibraryCollisionFunctions|SetDynamicMeshCollisionfromMesh :FromDynamicMesh _returnvalue_3 :ToDynamicMeshComponent _floordynamicmesh :Debug 0))

(fn ConstructionScript)